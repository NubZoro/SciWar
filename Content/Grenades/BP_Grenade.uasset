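; Grenade actor that explodes on a short timer or when its Sphere overlaps any actor other than player pawn 0.
; On overlap it destroys the other actor outright, with no damage call, while the timed explosion harms nothing.
; Both paths duplicate the same sequence: spawn a bubble particle effect, play an explosion sound, unhide Sphere1 and immediately destroy the grenade.
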(event OnComponentBeginOverlap(Sphere)
  (params (OverlappedComponent :type Primitive%20Component%20Object%20Reference) (OtherActor :type Actor%20Object%20Reference) (OtherComp :type Primitive%20Component%20Object%20Reference) (OtherBodyIndex :type Integer) (bFromSweep :type Boolean) (SweepResult :type Hit%20Result%20Structure%20%28by%20ref%29))
  (if (!= OtherActor (Game|Player|GetPlayerPawn 0))
    (Actor|DestroyActor OtherActor)
    (Effects|SpawnEmitteratLocation "/Game/Realistic_Starter_VFX_Pack_Vol2/Particles/Water/P_Bubbles_B.P_Bubbles_B" (Transformation|GetActorLocation))
    (Audio|PlaySoundatLocation "/Game/StarterContent/Audio/Explosion_Cue.Explosion_Cue" (Transformation|GetActorLocation) "0, 0, 0" 1.0 1.0 0.0 0 0 0 0)
    (Development|SetHiddeninGame (Variables|Default|GetSphere1) false false)
    (Actor|DestroyActor)))

(event EventBeginPlay
  (Utilities|FlowControl|Delay 1.5)
  (Utilities|IsValid self
    (:Is%20Valid
      (Effects|SpawnEmitteratLocation "/Game/Realistic_Starter_VFX_Pack_Vol2/Particles/Water/P_Bubbles_B.P_Bubbles_B" (Transformation|GetActorLocation))
      (Audio|PlaySoundatLocation "/Game/StarterContent/Audio/Explosion_Cue.Explosion_Cue" (Transformation|GetActorLocation) "0, 0, 0" 1.0 1.0 0.0 0 0 0 0)
      (Development|SetHiddeninGame (Variables|Default|GetSphere1) false false)
      (Actor|DestroyActor))))

(fn ConstructionScript)